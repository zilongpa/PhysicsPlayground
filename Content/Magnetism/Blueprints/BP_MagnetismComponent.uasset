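; Actor component that makes its owner act as a magnet, pushing or pulling nearby actors that also carry a magnetism component.
; Each tick, a capsule overlap within MagneticRange gathers those actors and applies force to their static meshes.
; Differing MagneticInfo attracts; matching flips the force, scaled by MagneticPush.
; Force scales with squared strength times moveability and inverse distance; ActivateComponent toggles activation and ticking.
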(event `self.ReceiveTick`
  (params (DeltaSeconds :type "Float (single-precision)"))
  ;[0.5649 0.6948 1] Updates the movement of the magnetic object
  (bind _influencedactors (`self.getActorsInRange`))
  (for _array_element _influencedactors
    (for _array_element_2 (`Actor.K2_GetComponentsByClass` _array_element "/Script/Engine.StaticMeshComponent")
      (if (== (`/Game/Magnetism/Blueprints/BP_MagnetismComponent.MagneticInfo` (`Actor.GetComponentByClass` (`self.GetOwner`) "BP_MagnetismComponent_C")) (`/Game/Magnetism/Blueprints/BP_MagnetismComponent.MagneticInfo` (`Actor.GetComponentByClass` _array_element "BP_MagnetismComponent_C")))
        (bind _returnvalue (- (`SceneComponent.K2_GetComponentLocation` _array_element_2) (`SceneComponent.K2_GetComponentLocation` (`Actor.GetComponentByClass` (`self.GetOwner`) "/Script/Engine.StaticMeshComponent"))))
        (bind _returnvalue_2 (* (`self.MagneticStrength`) (`/Game/Magnetism/Blueprints/BP_MagnetismComponent.MagneticMoveability` (`Actor.GetComponentByClass` _array_element "BP_MagnetismComponent_C"))))
        (bind _returnvalue_3 (* (`KismetMathLibrary.Normal` _returnvalue) (* (/ _returnvalue_2 (`KismetMathLibrary.VSize` _returnvalue)) _returnvalue_2 -1.0)))
        (`PrimitiveComponent.AddForce` _array_element_2 (* _returnvalue_3 (* (`self.MagneticPush`) -1.0)) "None" false)
        (else
          (`PrimitiveComponent.AddForce` _array_element_2 _returnvalue_3 "None" false))))))

(fn `activateComponent`
  (params (NewState :type Boolean))
  (`self.SetActive` NewState true)
  (`self.SetComponentTickEnabled` NewState))

(fn `getActorsInRange`
  (returns (InfluencedActors :type "Array of Actor Object Reference"))
  (locals (InfluencedActorsArray :type "Array of Actor Object Reference"))
  (bind _magneticrange (`self.MagneticRange`))
  ;[1 0.01819 0] Returns all actors which are in range to be influenced
  (bind _outactors (`KismetSystemLibrary.CapsuleOverlapActors` (`Actor.K2_GetActorLocation` (`self.GetOwner`)) _magneticrange _magneticrange (`|MakeArray` "ObjectTypeQuery1" "ObjectTypeQuery2" "ObjectTypeQuery3" "ObjectTypeQuery4" "ObjectTypeQuery5" :!type "EObjectTypeQuery Enum")))
  (for _array_element _outactors
    (if (and (!= (`self.GetOwner`) _array_element) (`KismetSystemLibrary.IsValid` (`Actor.GetComponentByClass` _array_element "BP_MagnetismComponent_C")))
      (`KismetArrayLibrary.Array_Add` (`local.InfluencedActorsArray`) _array_element)))
  (return (`local.InfluencedActorsArray`)))